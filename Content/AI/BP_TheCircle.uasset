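; BP_TheCircle is a shrinking-zone actor whose Walls component closes in over four timed phases.
; On BeginPlay it sizes the walls to MaxRadius, then waits WallShrinkInterval before each chained timeline.
; Each timeline's Scale feeds UpdateScale, which scales X and Y against MaxRadius while keeping height fixed.
; IsClosing flags active shrinking between pauses, and IsClosed is set during Phase4 updates, with IsClosing left true.
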(event EventBeginPlay
  (bind _maxradius (Variables|Default|GetMaxRadius))
  (Transformation|SetWorldScale3D (Variables|Default|GetWalls) (Math|Vector|MakeVector _maxradius _maxradius 1e+03))
  (Utilities|FlowControl|Delay (Variables|Default|GetWallShrinkInterval))
  (Variables|Default|SetIsClosing true)
  (bind _scale (Timeline|Phase%201 Play)
    (:Update
      (CallFunction|UpdateScale _scale))
    (:Finished
      (Variables|Default|SetIsClosing false)
      (Utilities|FlowControl|Delay (Variables|Default|GetWallShrinkInterval))
      (Variables|Default|SetIsClosing true)
      (bind _scale_2 (Timeline|Phase%202 Play)
        (:Update
          (CallFunction|UpdateScale _scale_2))
        (:Finished
          (Variables|Default|SetIsClosing false)
          (Utilities|FlowControl|Delay (Variables|Default|GetWallShrinkInterval))
          (Variables|Default|SetIsClosing true)
          (bind _scale_3 (Timeline|Phase%203 Play)
            (:Update
              (CallFunction|UpdateScale _scale_3))
            (:Finished
              (Variables|Default|SetIsClosing false)
              (Utilities|FlowControl|Delay (Variables|Default|GetWallShrinkInterval))
              (Variables|Default|SetIsClosing true)
              (bind _scale_4 (Timeline|Phase%204 Play)
                (:Update
                  (CallFunction|UpdateScale _scale_4)
                  (Variables|Default|SetisClosed true))))))))))

(fn ConstructionScript)

(fn UpdateScale
  (params (ScalePercent :type Float%20%28single-precision%29))
  (bind _maxradius (Variables|Default|GetMaxRadius))
  (bind _returnvalue (* ScalePercent _maxradius))
  (Transformation|SetWorldScale3D (Variables|Default|GetWalls) (Math|Vector|MakeVector _returnvalue _returnvalue 1e+03)))