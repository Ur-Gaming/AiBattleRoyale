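; BP_Pickup is an inventory pickup actor that displays an item's mesh with a nameplate widget.
; The construction script reads the item's data table row into Information, then Setup applies the mesh and passes the data to the ItemNameplate widget.
; BeginPlay pushes the data to the widget again.
; Tick turns the nameplate to face opposite the first player controller's forward vector, billboard-style.
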(event EventBeginPlay
  (CallFunction|SetUpNameplate)
  (CallFunction|Setup))

(event EventTick
  (params (DeltaSeconds :type Float%20%28single-precision%29))
  (CallFunction|UpdateRotation))

(fn ConstructionScript
  (bind _item (Variables|Default|GetItem))
  (bind (_datatable _rowname) (Utilities|Struct|BreakDataTableRowHandle _item))
  (bind _returnvalue (Utilities|GetDataTableRow _datatable _rowname)
    (:then
      (Variables|Default|SetInformation _returnvalue)
      (CallFunction|Setup))))

(fn Setup
  (Components|StaticMesh|SetStaticMesh (Variables|Default|GetModel) (.Model (Utilities|Struct|BreakST_Item (Variables|Default|GetInformation))))
  (bind _asitem_nameplate (Utilities|Casting|CastToItemNameplate (UserInterface|GetWidget (Variables|Default|GetNameplate))))
  (Variables|/Game/AI/InventorySystem/Interactables/ItemNameplate.ItemNameplate_C|SetInformation _asitem_nameplate (Variables|Default|GetInformation)))

(fn UpdateRotation
  (Transformation|SetWorldRotation (Variables|Default|GetNameplate) (Math|Conversions|RotationFromXVector (* (Transformation|GetActorForwardVector (Game|GetPlayerController 0)) -1.0)) false false))

(fn SetUpNameplate
  (bind _asitem_nameplate (Utilities|Casting|CastToItemNameplate (UserInterface|GetUserWidgetObject (Variables|Default|GetNameplate))))
  (Variables|/Game/AI/InventorySystem/Interactables/ItemNameplate.ItemNameplate_C|SetInformation _asitem_nameplate (Variables|Default|GetInformation)))