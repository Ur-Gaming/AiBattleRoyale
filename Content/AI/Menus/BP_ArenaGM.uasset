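; BP_ArenaGM runs a last-drone-standing arena match and declares the winner.
; On BeginPlay it stores the BP_TheCircle zone in the StandardInstance game instance and binds every BP_Drone1's destroy event.
; Each destruction rebuilds the drone list without the destroyed actor.
; Tick polls that list and, once one drone remains, shows the cursor, clears widgets and displays the game instance's victory screen with that drone's name.
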(event Custom|Update%20Player%20List
  (params (DestroyedActor :type Actor%20Object%20Reference))
  (bind _outactors (Actor|GetAllActorsOfClass "/Game/AI/BP_Drone1.BP_Drone1_C"))
  (bind _output_get (Variables|Default|SetActorArray _outactors))
  (bind _asbp_drone_1 (Utilities|Casting|CastToBP_Drone1 DestroyedActor))
  (Utilities|Array|RemoveItem _output_get _asbp_drone_1))

(event Custom|Check%20Drones
  (params (DestroyedActor :type Actor%20Object%20Reference))
  ;[1 1 1] Find, bind, and set drones
  (CallFunction|UpdatePlayerList DestroyedActor))

(event EventBeginPlay
  ;[1 1 1] Find and set zone
  (bind _returnvalue (Actor|GetActorOfClass "/Game/AI/BP_TheCircle.BP_TheCircle_C"))
  (bind _asstandard_instance (Utilities|Casting|CastToStandardInstance (Game|GetGameInstance)))
  (bind _output_get (Variables|/Game/AI/Menus/StandardInstance.StandardInstance_C|SetZone _asstandard_instance _returnvalue))
  (Utilities|IsValid _output_get
    (:Is%20Valid
      (Development|PrintString "Zone Found"))
    (:Is%20Not%20Valid
      (Development|PrintString "Could not find instance of the zone")))
  ;[1 1 1] Find, bind, and set drones
  (bind _outactors (Actor|GetAllActorsOfClass "/Game/AI/BP_Drone1.BP_Drone1_C"))
  (bind _output_get_2 (Variables|Default|SetActorArray _outactors))
  (for _array_element _output_get_2
    (if (Utilities|IsValid _array_element)
      (Game|BindEventtoOnDestroyed _array_element (delegate Custom|Check%20Drones)))))

(event EventTick
  (params (DeltaSeconds :type Float%20%28single-precision%29))
  (bind _returnvalue (Game|GetPlayerController 0))
  (if (and (== (Utilities|Array|Length (Variables|Default|GetActorArray)) 1) (not (Variables|Default|GetIsGameOver)))
    (if (not (Variables|/Script/Engine.PlayerController|GetbShowMouseCursor _returnvalue))
      (Variables|/Script/Engine.PlayerController|SetbShowMouseCursor _returnvalue true))
    (Viewport|RemoveAllWidgets)
    (bind _asstandard_instance (Utilities|Casting|CastToStandardInstance (Game|GetGameInstance)))
    (Default|SetWinText (Variables|/Game/AI/Menus/StandardInstance.StandardInstance_C|GetVictoryScreenWidget _asstandard_instance) (Variables|/Game/AI/BP_Drone1.BP_Drone1_C|GetName (Utilities|Array|Get(acopy) (Variables|Default|GetActorArray))))
    (UserInterface|Viewport|AddtoViewport (Variables|/Game/AI/Menus/StandardInstance.StandardInstance_C|GetVictoryScreenWidget _asstandard_instance) 0)
    (Variables|Default|SetIsGameOver true)))

(fn ConstructionScript)