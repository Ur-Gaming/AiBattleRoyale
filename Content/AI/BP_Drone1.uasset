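; BP_Drone1 is an AI drone character with health, a nameplate widget, and an attack that only damages other BP_Drone1 instances.
; Leaving BP_TheCircle starts a looping timer that applies the zone damage read from StandardInstance, and re-entering clears it.
; AnyDamage routes all hits into ReceiveDamage, which lowers Health and destroys the drone at zero.
; The IsDead and OnDeath branch in Attack is disconnected.
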(event Custom|OnDeath
  (Actor|DestroyActor))

(event Custom|Begin%20ZoneDamage
  (bind _returnvalue (Utilities|Time|SetTimerbyEvent (delegate Custom|Receive%20ZoneDamage) (Variables|Default|GetZoneDamageDelay) true))
  (Variables|Default|SetZoneDamageTimer _returnvalue))

(event Custom|Receive%20ZoneDamage
  (bind _asstandard_instance (Utilities|Casting|CastToStandardInstance (Game|GetGameInstance)))
  (Game|Damage|ApplyDamage self (Variables|/Game/AI/BP_TheCircle.BP_TheCircle_C|GetZoneDamage (Variables|/Game/AI/Menus/StandardInstance.StandardInstance_C|GetZone _asstandard_instance)) 0 (Variables|/Game/AI/Menus/StandardInstance.StandardInstance_C|GetZone _asstandard_instance))
  (Utilities|FlowControl|Delay (Variables|Default|GetZoneDamageDelay)))

(event Custom|End%20ZoneDamage
  (Utilities|Time|ClearandInvalidateTimerbyHandle (Variables|Default|GetZoneDamageTimer)))

(event EventBeginPlay
  (Variables|Default|SetHealth (Variables|Default|GetMaxHealth))
  (CallFunction|NameplateSetup))

(event Collision|EventActorBeginOverlap
  (params (OtherActor :type Actor%20Object%20Reference))
  (Utilities|Casting|CastToBP_TheCircle OtherActor)
  (Variables|Default|SetTakingZoneDamage false)
  (CallFunction|EndZoneDamage))

(event Collision|EventActorEndOverlap
  (params (OtherActor :type Actor%20Object%20Reference))
  (Utilities|Casting|CastToBP_TheCircle OtherActor)
  (Variables|Default|SetTakingZoneDamage true)
  (CallFunction|BeginZoneDamage))

(event Game|Damage|EventAnyDamage
  (params (Damage :type Float%20%28single-precision%29) (DamageType :type Damage%20Type%20Object%20Reference) (InstigatedBy :type Controller%20Object%20Reference) (DamageCauser :type Actor%20Object%20Reference))
  (CallFunction|ReceiveDamage Damage))

(fn ConstructionScript)

(fn Attack
  (params (Enemy :type Actor%20Object%20Reference))
  (bind _asbp_drone_1 (Utilities|Casting|CastToBP_Drone1 Enemy))
  (Game|Damage|ApplyDamage _asbp_drone_1 (Variables|Default|GetDamage) (Pawn|GetController) self))

(fn NameplateSetup
  (bind _asnameplate (Utilities|Casting|CastToNameplate (UserInterface|GetUserWidgetObject (Variables|Default|GetNameplate))))
  (Variables|/Game/AI/Nameplate.Nameplate_C|SetCharacter _asnameplate self))

(fn ReceiveDamage
  (params (Damage :type Float%20%28single-precision%29))
  (bind _output_get (Variables|Default|SetHealth (- (Variables|Default|GetHealth) Damage)))
  (if (<= _output_get 0.0)
    (Actor|DestroyActor)))